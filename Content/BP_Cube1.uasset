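; BP_Cube1 is an actor that steps forward along world X when W is pressed.
; The key press calls the Server_Moveer event, named as a server call, which runs MoveForwardSetBackCreatorX8 to add a small fixed offset without sweeping for collision.
; A separate MoveForward function makes a far larger jump the same way, but nothing in this Blueprint calls it.
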(event Custom|Server_Moveer
  (CallFunction|MoveForwardSetBackCreatorX=8))

(event EventBeginPlay)

(event Collision|EventActorBeginOverlap
  (params (OtherActor :type Actor%20Object%20Reference)))

(event Input|KeyboardEvents|W
  (params (Key :type Key%20Structure :default "None"))
  (:Pressed
    (CallFunction|ServerMoveer)))

(fn ConstructionScript)

(fn MoveForward
  (bind _returnvalue (Transformation|GetActorLocation))
  (bind _returnvalue_2 (+ _returnvalue "20000.000000,0.000000,0.000000"))
  (Transformation|SetActorLocation _returnvalue_2 false false)
  (return _returnvalue_2))

(fn MoveForwardSetBackCreatorX=8
  (bind _returnvalue (Transformation|GetActorLocation))
  (bind _returnvalue_2 (+ _returnvalue "8.000000,0.000000,0.000000"))
  (Transformation|SetActorLocation _returnvalue_2 false false)
  (return _returnvalue_2))