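; BP_Cube3 is a cube actor that demonstrates client-side prediction and server correction when W moves it forward.
; Without authority, it moves 10 units immediately, turns red and calls the server, which deliberately moves a shorter 8 units to create a mismatch.
; The server sends a position through Client_Mover, which clears the prediction state and restores the basic material.
; Tick then keeps interpolating the cube toward that server target.
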(event Custom|Server_Moveer
  (bind _resulting_position (CallFunction|MoveForwardSetBackCreatorX=8))
  (CallFunction|ClientMover _resulting_position))

(event Custom|Client_Mover
  (params (ActualPosi :type Vector))
  (Variables|Default|SetTargetServerPosition ActualPosi)
  (Variables|Default|SetDoneDoingAll? true)
  (Variables|Default|SetIsPredictionActive? false))

(event EventBeginPlay
  (CallFunction|MaterialSet))

(event Collision|EventActorBeginOverlap
  (params (OtherActor :type Actor%20Object%20Reference)))

(event EventTick
  (params (DeltaSeconds :type Float%20%28single-precision%29))
  (if (Variables|Default|GetDoneDoingAll?)
    (Transformation|SetActorLocation (Math|Interpolation|VInterpTo (Transformation|GetActorLocation) (Variables|Default|GetTargetServerPosition) DeltaSeconds 25.0) false false))
  (if (Variables|Default|GetIsPredictionActive?)
    (Rendering|Material|SetMaterial (Variables|Default|GetCube) 0 "/Engine/BasicShapes/Red.Red")
    (else
      (Rendering|Material|SetMaterial (Variables|Default|GetCube) 0 "/Engine/BasicShapes/BasicShapeMaterial.BasicShapeMaterial"))))

(event Input|KeyboardEvents|W
  (params (Key :type Key%20Structure :default "None"))
  (:Pressed
    (if (Ability|HasAuthority)
      (CallFunction|MoveForward)
      (else
        (bind _resulting_position (CallFunction|MoveForward))
        (Variables|Default|SetIsPredictionActive? true)
        (Development|PrintString "Changed to red")
        (CallFunction|ServerMoveer)
        (Variables|Default|SetWrong%20Posi _resulting_position)))))

(fn ConstructionScript)

(fn MoveForward
  (bind _returnvalue (Transformation|GetActorLocation))
  (bind _returnvalue_2 (+ _returnvalue "10.000000,0.000000,0.000000"))
  (Transformation|SetActorLocation _returnvalue_2 false false)
  (return _returnvalue_2))

(fn MoveForwardSetBackCreatorX=8
  (bind _returnvalue (Transformation|GetActorLocation))
  (bind _returnvalue_2 (+ _returnvalue "8.000000,0.000000,0.000000"))
  (Transformation|SetActorLocation _returnvalue_2 false false)
  (Development|PrintString (Utilities|String|ToString(Vector) _returnvalue_2))
  (return _returnvalue_2))

(fn MaterialSet
  (Rendering|Material|SetMaterial (Variables|Default|GetCube) 0 "/Engine/BasicShapes/BasicShapeMaterial.BasicShapeMaterial")
  (Development|PrintString "Setted the material"))